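; BP_Rifle_Character is a first-person rifle character with arms, a weapon and a camera.
; Its construction script attaches the Weapon component to the R_GunSocket socket on the Arms.
; The MoveForward and MoveRight axis events are empty, and the HMD-aware movement nodes are disconnected, so this graph applies no movement.
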(event Input|AxisEvents|InputAxisMoveForward
  (params (AxisValue :type Float%20%28single-precision%29))
  ;[1 1 1] Movement Input - If using an HMD, movement is based off HMD location. Use with key bindings
)

(event Input|AxisEvents|InputAxisMoveRight
  (params (AxisValue :type Float%20%28single-precision%29))
  ;[1 1 1] Movement Input - If using an HMD, movement is based off HMD location. Use with key bindings
)

(fn ConstructionScript
  (Transformation|AttachComponentToComponent (Variables|Default|GetWeapon) (Variables|Default|GetArms) "R_GunSocket" "KeepRelative" "KeepRelative" "KeepRelative" true))